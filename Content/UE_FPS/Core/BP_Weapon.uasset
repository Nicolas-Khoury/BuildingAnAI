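; BP_Weapon is a weapon actor for an FPS shooter character, with empty StartFire and StopFire events that define the firing interface.
; BeginPlay caches the owning BP_ShooterCharacter, and the construction script turns off auto-activation of the shoot sound, muzzle flash and camera shake source.
; SetActive toggles visibility and ticking, sets the mesh to no collision in either state, and calls StopFire.
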(event Custom|StopFire
  ;[1 1 1] Declare Start and Stop Fire Events
)

(event Custom|StartFire
  ;[1 1 1] Declare Start and Stop Fire Events
)

(event EventBeginPlay
  ;[1 1 1] Save Reference to Player
  (bind _asbp_shooter_character (Utilities|Casting|CastToBP_ShooterCharacter (Components|GetOwner)))
  (Variables|Default|SetOwningCharacter _asbp_shooter_character))

(fn ConstructionScript
  ;[1 1 1] Stop Automatic Audio Play
  (Components|Activation|SetAutoActivate (Variables|Default|GetShootSound) false)
  ;[1 1 1] Stop Automatic FX Start
  (Components|Activation|SetAutoActivate (Variables|Default|GetMuzzleFlash) false)
  ;[1 1 1] Stop Automatic Camera Shake Play
  (Components|Activation|SetAutoActivate (Variables|Default|GetCameraShakeSource) false))

(fn SetActive
  (params (bActive :type Boolean))
  (Rendering|SetActorHiddenInGame (not bActive))
  (Actor|Tick|SetActorTickEnabled bActive)
  (Collision|SetCollisionEnabled (Variables|Default|GetMesh) (select bActive "NoCollision" "NoCollision"))
  (CallFunction|StopFire))