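; Automatic rifle child weapon that fires hitscan shots on a looping timer derived from FireRate, starting with an immediate shot.
; Each shot traces from the muzzle toward the camera's aim point at Range and applies point damage on hit.
; Start and stop toggle the first-person fire montage, looping sound, muzzle flash and camera shake, with a short delay on stop.
; The construction script assigns the rifle's type and effect assets.
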(event Custom|StartFX
  (bind _owningcharacter (Variables|Default|GetOwningCharacter))
  (Utilities|IsValid _owningcharacter
    (:Is%20Valid
      (Animation|Montage|PlayMontage (Variables|/Game/UE_FPS/Core/BP_ShooterCharacter.BP_ShooterCharacter_C|GetMesh1P _owningcharacter) (Variables|Default|GetFireMontage)
        (:then
          _)))
    (:Is%20Not%20Valid
      _))
  (Components|Activation|SetActive (Variables|Default|GetShootSound) true false)
  (Components|Activation|SetActive (Variables|Default|GetMuzzleFlash) true false)
  (CameraShake|Start (Variables|Default|GetCameraShakeSource)))

(event Custom|StopFX
  (bind _owningcharacter (Variables|Default|GetOwningCharacter))
  (Utilities|IsValid _owningcharacter
    (:Is%20Valid
      (Animation|Montage|MontageStop (Components|SkeletalMesh|GetAnimInstance (Variables|/Game/UE_FPS/Core/BP_ShooterCharacter.BP_ShooterCharacter_C|GetMesh1P _owningcharacter)) 0.1 "/Game/Animations/FPP_Animations/HerroFPP_RifleFire_Montage.HerroFPP_RifleFire_Montage"))
    (:Is%20Not%20Valid
      _))
  (Components|Activation|SetActive (Variables|Default|GetShootSound) false false)
  (Components|Activation|SetActive (Variables|Default|GetMuzzleFlash) false false)
  (CameraShake|StopAllCameraShakes (Variables|Default|GetCameraShakeSource) false))

(event Custom|Fire%20Bullet
  (bind _owningcharacter (Variables|Default|GetOwningCharacter))
  (bind _playercamera (Variables|/Game/UE_FPS/Core/BP_ShooterCharacter.BP_ShooterCharacter_C|GetPlayerCamera _owningcharacter))
  ;[1 1 1] Spawn Bullet
  (bind (_outhit _returnvalue) (Collision|LineTraceByChannel (Transformation|GetWorldLocation (Variables|Default|GetMuzzleArrow)) (+ (Transformation|GetWorldLocation _playercamera) (* (Math|Vector|GetForwardVector _playercamera) (Variables|Default|GetRange))) "TraceTypeQuery1" false (Utilities|Array|MakeArray _owningcharacter) "None"))
  (if _returnvalue
    (Game|Damage|ApplyPointDamage (.HitActor (Collision|BreakHitResult _outhit)) 5.0 (.ImpactNormal (Collision|BreakHitResult _outhit)) _outhit (Pawn|GetController (Variables|Default|GetOwningCharacter)) self)))

(event EventStartFire
  (|CallParentFunction)
  ;[1 1 1] Setup and start firing timer
  (bind _returnvalue (Utilities|Time|SetTimerbyEvent (delegate Custom|Fire%20Bullet) (Math|Float|SafeDivide 1.0 (Variables|Default|GetFire%20Rate)) true))
  (Variables|Default|SetFiring%20Timer _returnvalue)
  (CallFunction|FireBullet)
  (CallFunction|StartFX))

(event EventStopFire
  (|CallParentFunction)
  ;[1 1 1] Stop Firing Timer
  (Utilities|Time|ClearandInvalidateTimerbyHandle (Variables|Default|GetFiring%20Timer))
  (Audio|Components|Audio|Stop (Variables|Default|GetShootSound))
  (Utilities|FlowControl|Delay 0.1)
  (CallFunction|StopFX))

(fn ConstructionScript
  (|CallParentFunction)
  (Variables|Default|SetType "NewEnumerator0")
  (Variables|Default|SetFireMontage "/Game/Animations/FPP_Animations/HerroFPP_RifleFire_Montage.HerroFPP_RifleFire_Montage")
  (Audio|Components|Audio|SetSound (Variables|Default|GetShootSound) "/Game/Sounds/Weapons/AssultRifle/SCue_AR_Shoot_LP.SCue_AR_Shoot_LP")
  (Effects|Components|ParticleSystem|SetTemplate (Variables|Default|GetMuzzleFlash) "/Game/Effects/ParticleSystems/Weapons/AssaultRifle/Muzzle/P_AssaultRifle_MF.P_AssaultRifle_MF")
  (Variables|/Script/Engine.CameraShakeSourceComponent|SetCameraShake (Variables|Default|GetCameraShakeSource) "/Game/UE_FPS/Core/WeapGun_FireCameraShake.WeapGun_FireCameraShake_C"))